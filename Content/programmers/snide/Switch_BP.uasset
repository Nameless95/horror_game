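; Switch Blueprint that toggles a referenced point light's visibility when its Interactobj event fires.
; HitRay1 and RayGone events enable and disable player 0's input on the actor, print debug text and set InRange, which is never read.
; Interactobj branches on LightOn, but both branches toggle visibility and write back the same value, so the flag never changes.
; The box overlap events are empty.
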(event `self.Box.OnComponentBeginOverlap`
  (params (OverlappedComponent :type "PrimitiveComponent Object Reference") (OtherActor :type "Actor Object Reference") (OtherComp :type "PrimitiveComponent Object Reference") (OtherBodyIndex :type Integer) (bFromSweep :type Boolean) (SweepResult :type "HitResult Structure (by ref)")))

(event `self.hit_ray_1`
  (`self.EnableInput` (`GameplayStatics.GetPlayerController` 0))
  (`KismetSystemLibrary.PrintText` "OverLapping")
  (set `self.InRange` true))

(event `self.ray gone`
  (`self.DisableInput` (`GameplayStatics.GetPlayerController` 0))
  (`KismetSystemLibrary.PrintText` "Not OverLapping")
  (set `self.InRange` false))

(event `self.Box.OnComponentEndOverlap`
  (params (OverlappedComponent :type "PrimitiveComponent Object Reference") (OtherActor :type "Actor Object Reference") (OtherComp :type "PrimitiveComponent Object Reference") (OtherBodyIndex :type Integer)))

(event `self.interactobj`
  (if (`self.LightOn`)
    (`SceneComponent.ToggleVisibility` (`Actor.RootComponent` (`self.pointLight`)) false)
    (set `self.LightOn` true)
    (else
      (`SceneComponent.ToggleVisibility` (`Actor.RootComponent` (`self.pointLight`)) false)
      (set `self.LightOn` false))))

(fn `UserConstructionScript`)