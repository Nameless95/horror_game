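; Lightning effect actor that fires a strike in the player's view every few seconds.
; Each strike moves the actor to a random point ahead of the player, yawed toward them, and plays 2D thunder.
; A timeline animates the lightning plane's material parameters for shape and emission.
; Shortly after, the post-process volume briefly switches to a fixed manual exposure for a screen flash, then restores the saved compensation.
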(event `self.ReceiveBeginPlay`
  (bind _pp_volume (`self.PP_volume`))
  (`KismetSystemLibrary.Delay` (`KismetMathLibrary.RandomFloatInRange` 6.0 8.0) :!label _label)
  (`self.Strike`)
  (`KismetSystemLibrary.Delay` 0.2)
  (bind _output_get (set `self.Original Exposure Compensation` (`.AutoExposureBias` (break `PostProcessSettings` (`PostProcessVolume.Settings` _pp_volume)))))
  (set `PostProcessVolume.Settings` (make `PostProcessSettings` :`AutoExposureMethod` "AEM_Manual" :`AutoExposureBias` 11.0) _pp_volume)
  (`KismetSystemLibrary.Delay` 0.2)
  (set `PostProcessVolume.Settings` (make `PostProcessSettings` :`AutoExposureMethod` "AEM_Manual" :`AutoExposureBias` _output_get) _pp_volume)
  (goto _label))

(event `Strike`
  (bind _lighting_plane (`self.Lighting_plane`))
  (bind _returnvalue (`Controller.GetControlRotation` (`GameplayStatics.GetPlayerController` 0)))
  (bind _returnvalue_2 (`self.K2_GetActorLocation` (`GameplayStatics.GetPlayerCharacter` 0)))
  (bind _returnvalue_3 (+ (* (`KismetMathLibrary.GetForwardVector` _returnvalue) (`KismetMathLibrary.RandomFloatInRange` 2000.0 3000.0)) _returnvalue_2 (* (`KismetMathLibrary.GetRightVector` _returnvalue) (`KismetMathLibrary.RandomFloatInRange` -3000.0 3000.0)) (0.0 0.0 600.0)))
  (bind (_returnvalue_roll _returnvalue_pitch _returnvalue_yaw) (`KismetMathLibrary.BreakRotator` (`KismetMathLibrary.FindLookAtRotation` _returnvalue_3 _returnvalue_2)))
  (`self.K2_SetActorLocationAndRotation` _returnvalue_3 (`KismetMathLibrary.MakeRotator` 0.0 0.0 _returnvalue_yaw))
  (`GameplayStatics.PlaySound2D` "/Game/Maps/Exterior/FX/Audio/Thunder_Strike.Thunder_Strike" 1.0 1.0 0.0 null null)
  (bind (_direction _y) (`Timeline|Lighting_strike` :!via `PlayFromStart`)
    (:`Update`
      (`MeshComponent.SetVectorParameterValueOnMaterials` _lighting_plane "Y" (`KismetMathLibrary.Conv_DoubleToVector` _y))
      (`MeshComponent.SetVectorParameterValueOnMaterials` _lighting_plane "Emission" (`KismetMathLibrary.Conv_DoubleToVector` (* (+ _y 1.0) 50.0))))))

(fn `UserConstructionScript`)